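; Behemoth character Blueprint that handles HUD panel toggles and seeds the character's starting inventory.
; Inventory and character-info events cast the player HUD to W_PlayerHUD and use FlipFlops to show or hide each panel, refreshing the inventory when shown.
; BeginPlay adds two DT_Items rows to the InventoryComponent, the second lookup running only if the first succeeds.
; A test key (X) applies damage to the character itself.
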(event `self.ToggleInventory`
  ;[1 1 1] Inventory Toggle
  (bind _asw_player_hud (cast `/Game/Blueprints/UI/MainHUD/W_PlayerHUD` (`self.PlayerHUD`)))
  (`/Engine/EditorBlueprintResources/StandardMacros.FlipFlop`
    (:`A`
      (bind _w_inventory (`/Game/Blueprints/UI/MainHUD/W_PlayerHUD.W_Inventory` _asw_player_hud))
      (`Widget.SetVisibility` _w_inventory "Visible")
      (`/Game/Blueprints/UI/Inventory/W_Inventory.RefreshInventory` _w_inventory))
    (:`B`
      (`Widget.SetVisibility` _w_inventory "Hidden"))))

(event `self.ToggleCharacterInfo`
  ;[1 1 1] Character Info Toggle
  (bind _asw_player_hud (cast `/Game/Blueprints/UI/MainHUD/W_PlayerHUD` (`self.PlayerHUD`)))
  (`/Engine/EditorBlueprintResources/StandardMacros.FlipFlop`
    (:`A`
      (bind _w_charactersheetui (`/Game/Blueprints/UI/MainHUD/W_PlayerHUD.W_CharacterSheetUI` _asw_player_hud))
      (`Widget.SetVisibility` _w_charactersheetui "Visible"))
    (:`B`
      (`Widget.SetVisibility` _w_charactersheetui "Hidden"))))

(event `Key|X`
  (params (Key :type "Key Structure"))
  ;[1 1 1] Testing
  (:`Pressed`
    (`GameplayStatics.ApplyDamage` self 10.0 null self)))

(event `self.ReceiveBeginPlay`
  ;[1 1 1] Testing
  (bind _returnvalue (`|GetDataTableRow` "/Game/Blueprints/Data/DT_Items.DT_Items" "2")
    (:`then`
      (`BHInventoryComponent.AddToInventory` (`self.InventoryComponent`) _returnvalue 1)
      (bind _returnvalue_2 (`|GetDataTableRow` "/Game/Blueprints/Data/DT_Items.DT_Items" "1")
        (:`then`
          (`BHInventoryComponent.AddToInventory` (`self.InventoryComponent`) _returnvalue_2 1))))))

(fn `UserConstructionScript`)